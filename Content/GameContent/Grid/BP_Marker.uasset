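; BP_Marker is a grid marker that shows placement feedback by swapping the material on its mesh.
; ActivateMarker takes a placement type (Place, Destroy or Rotate), applies the matching placing, destroying or moving material, and sets the Activated flag.
; DeactivateMarker restores the default material and clears the flag.
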(event Custom|ActivateMarker
  (params (Placement%20Type :type ENUM_PlaceMode%20Enum :default "NewEnumerator0"))
  ;[0.5795 0.2586 1 1 34] HANDLE ACTIVATION STATUS
  (switch Utilities|FlowControl|Switch|SwitchonENUM_PlaceMode Placement%20Type
    (:NewEnumerator0
      (Rendering|Material|SetMaterial (Variables|Default|GetMesh) 0 (Variables|Default|GetPlacingMaterial))
      (Variables|Default|SetActivated true))
    (:NewEnumerator1
      (Rendering|Material|SetMaterial (Variables|Default|GetMesh) 0 (Variables|Default|GetDestroyingMaterial))
      (Variables|Default|SetActivated true))
    (:NewEnumerator2
      (Rendering|Material|SetMaterial (Variables|Default|GetMesh) 0 (Variables|Default|GetMovingMaterial))
      (Variables|Default|SetActivated true))))

(event Custom|DeactivateMarker
  ;[0.5795 0.2586 1 1 34] HANDLE ACTIVATION STATUS
  (Rendering|Material|SetMaterial (Variables|Default|GetMesh) 0 (Variables|Default|GetDefaultMaterial))
  (Variables|Default|SetActivated false))

(fn ConstructionScript)