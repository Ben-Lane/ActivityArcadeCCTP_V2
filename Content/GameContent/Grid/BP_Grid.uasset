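; BP_Grid is a tile placement grid that highlights the hovered tile and previews the item chosen through the UI.
; The construction script sizes the plane and finds the starting tile; BeginPlay registers with BP_TopDownController and spawns marker and item child actors per tile.
; UpdateTileSelected converts hit locations to row-major child indices, previewing according to edit mode and reverting tiles left behind.
; Input mode events toggle marker visibility.
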(event Custom|ChangeDraggedItem
  (params (ItemType :type ENUM_ItemNames%20Enum :default "NewEnumerator0"))
  ;[1 0.4623 0.2193 1 42] UPDATE DRAGGED ITEM (USING UI)
  (Variables|Default|SetDraggedItem ItemType))

(event EventBeginPlay
  ;[0 0 0 1 42] SETUP GRID OBJECT SPAWNING (X IS UP, Y IS DOWN)
  (bind _asbp_top_down_controller (Utilities|Casting|CastToBP_TopDownController (Game|GetPlayerController 0)))
  (Variables|/Game/TopDown/Blueprints/BP_TopDownController.BP_TopDownController_C|SetGridObjectReference _asbp_top_down_controller self)
  (EventDispatchers|BindEventtoUpdateDraggedItem _asbp_top_down_controller (delegate Custom|ChangeDraggedItem))
  (CallFunction|GenerateTileMarkers)
  (Rendering|SetVisibility (Variables|Default|GetGridTileMarkers) false true))

(event EventChangeItem
  (params (ItemType :type ENUM_ItemNames%20Enum :default "NewEnumerator0"))
  ;[1 1 1 1 34] UPDATES DRAGGED ITEM SELECETED + EDIT MODE
  (Variables|Default|SetDraggedItem ItemType))

(event EventChangePlacementMode
  (params (PlaceMode :type ENUM_PlaceMode%20Enum :default "NewEnumerator0"))
  ;[1 1 1 1 34] UPDATES DRAGGED ITEM SELECETED + EDIT MODE
  (Variables|Default|SetEditMode PlaceMode))

(event EventInputMode-Edit
  ;[1 0.1458 0.1458 1 32] TOGGLE INPUT MODE (MAKE MARKERS INVISIBLE)
  (Rendering|SetVisibility (Variables|Default|GetGridTileMarkers) true true))

(event EventInputMode-Gameplay
  ;[1 0.1458 0.1458 1 32] TOGGLE INPUT MODE (MAKE MARKERS INVISIBLE)
  (Rendering|SetVisibility (Variables|Default|GetGridTileMarkers) false true))

(fn ConstructionScript
  (bind _gridplane (Variables|Default|GetGridPlane))
  ;[0.2874 1 0.5502] FLIP TO ALIGN PERSPECTIVE
  (Variables|Default|SetGridSize (Math|Vector2D|MakeVector2D (.y (Variables|Default|GetGridSize)) (.x (Variables|Default|GetGridSize))))
  ;[1 1 1] MAKE PLANE SIZE WANTED
  (Transformation|SetRelativeScale3D _gridplane (Math|Vector|MakeVector (.x (Variables|Default|GetGridSize)) (.y (Variables|Default|GetGridSize)) (.z (Variables|/Script/Engine.SceneComponent|GetRelativeScale3D _gridplane))))
  (CallFunction|FindStartingTile))

(fn FindStartingTile
  (if (== (/ (.x (Variables|Default|GetGridSize)) 2.0) 0.0)
    ;[0.149 0.2353 1] ODD GRID SIZE "X"
    (LocalVariables|SetStartingX (- (.x (Transformation|GetWorldLocation (Variables|Default|GetGridPlane))) (* (Math|Float|Truncate (/ (.x (Variables|Default|GetGridSize)) 2.0)) (.x (Variables|Default|GetTileSize)))))
    (else
      ;[0.149 0.2353 1] EVEN GRID SIZE "X"
      (LocalVariables|SetStartingX (- (.x (Transformation|GetWorldLocation (Variables|Default|GetGridPlane))) (* (/ (- (.x (Variables|Default|GetGridSize)) 1.0) 2.0) (.x (Variables|Default|GetTileSize)))))))
  (if (== (/ (.y (Variables|Default|GetGridSize)) 2.0) 0.0)
    ;[1 0.5255 0.1647] ODD GRID SIZE "Y"
    (LocalVariables|SetStartingY (- (.y (Transformation|GetWorldLocation (Variables|Default|GetGridPlane))) (* (Math|Float|Truncate (/ (.y (Variables|Default|GetGridSize)) 2.0)) (.y (Variables|Default|GetTileSize)))))
    (else
      ;[1 0.5255 0.1647] EVEN GRID SIZE "Y"
      (LocalVariables|SetStartingY (- (.y (Transformation|GetWorldLocation (Variables|Default|GetGridPlane))) (* (/ (- (.y (Variables|Default|GetGridSize)) 1.0) 2.0) (.y (Variables|Default|GetTileSize)))))))
  (Variables|Default|SetStartingTilePosition (Math|Vector2D|MakeVector2D (LocalVariables|GetStartingX) (LocalVariables|GetStartingY))))

(fn GenerateTileMarkers
  ;[0.7814 0.2419 1 1 58] CREATE GRID OF MARKERS FOR EACH TILE
  (LocalVariables|SetNextTilePosition (Variables|Default|GetStartingTilePosition))
  (for _index (range 0 (- (Math|Float|Truncate (.y (Variables|Default|GetGridSize))) 1))
    (LocalVariables|SetIndexY _index)
    (for _index_2 (range 0 (- (Math|Float|Truncate (.x (Variables|Default|GetGridSize))) 1))
      (LocalVariables|SetIndexX _index_2)
      (bind _returnvalue (AddComponent|AddChildActorComponent false))
      (Transformation|AttachComponentToComponent _returnvalue (Variables|Default|GetGridTileMarkers) "None" "KeepRelative" "KeepRelative" "KeepRelative" true)
      (ChildActorComponent|SetChildActorClass _returnvalue "/Game/GameContent/Grid/BP_Marker.BP_Marker_C")
      (bind _asbp_marker (Utilities|Casting|CastToBP_Marker (Variables|/Script/Engine.ChildActorComponent|GetChildActor _returnvalue)))
      (Transformation|SetActorLocation _asbp_marker (Math|Vector|MakeVector (.x (LocalVariables|GetNextTilePosition)) (.y (LocalVariables|GetNextTilePosition)) (.z (Transformation|GetActorLocation _asbp_marker))) false false)
      (Variables|/Game/GameContent/Grid/BP_Marker.BP_Marker_C|SetGridPos _asbp_marker (Math|Vector2D|MakeVector2D (Math|Conversions|ToFloat(Integer) (LocalVariables|GetIndexX)) (Math|Conversions|ToFloat(Integer) (LocalVariables|GetIndexY))))
      (Collision|SetActorEnableCollision _asbp_marker false)
      ;;[1 1 1 1 20] CREATES ITEM FOR CHANGING IN GRID
      (CallFunction|CreateBlankItem (Math|Vector|MakeVector (.x (LocalVariables|GetNextTilePosition)) (.y (LocalVariables|GetNextTilePosition)) (.z (Transformation|GetActorLocation _asbp_marker))))
      (LocalVariables|SetNextTilePosition (Math|Vector2D|MakeVector2D (+ (.x (LocalVariables|GetNextTilePosition)) (.x (Variables|Default|GetTileSize))) (.y (LocalVariables|GetNextTilePosition)))))
    (LocalVariables|SetNextTilePosition (Math|Vector2D|MakeVector2D (.x (Variables|Default|GetStartingTilePosition)) (+ (.y (LocalVariables|GetNextTilePosition)) (.y (Variables|Default|GetTileSize)))))))

(fn CurrentInputMode)

(fn UpdateTileSelected
  (params (HitLocation :type Vector))
  (bind _tilesize (Variables|Default|GetTileSize))
  (bind _gridsize (Variables|Default|GetGridSize))
  (bind _startingtileposition (Variables|Default|GetStartingTilePosition))
  (bind _tilesize_2 (Variables|Default|GetTileSize))
  ;[1 0.8462 0 1 66] FIND MARKER POSITION IN GRID
  (bind _output_get (LocalVariables|SetTileInGrid (Math|Vector2D|MakeVector2D (Math|Conversions|ToFloat(Integer) (- (Math|Float|Floor (/ (.x HitLocation) (.x _tilesize))) (Math|Float|Floor (/ (.x _startingtileposition) (.x _tilesize_2))))) (Math|Conversions|ToFloat(Integer) (- (Math|Float|Floor (/ (.y HitLocation) (.y _tilesize))) (Math|Float|Floor (/ (.y _startingtileposition) (.y _tilesize_2))))))))
  ;[0 0 0 1 34] ENSURE MOUSE IS HOVERING THE BOARD
  (if (Math|Boolean|ORBoolean (< (.x _output_get) 0.0) (< (.y _output_get) 0.0) (>= (.x _output_get) (.x _gridsize)) (>= (.y _output_get) (.y _gridsize)))
    ;[1 0 0] DEACTIVATE TILE WHEN LEAVING GRID BOUNDS
    (CallFunction|DeactivateSelectedTile)
    (CallFunction|RevertItemVisual (Variables|Default|GetSelectedTile))
    (else
      ;[0.08157 1 0 1 66] TurnMarkerOn
      (bind _aschild_actor_component (Utilities|Casting|CastToChildActorComponent (Components|GetChildComponent (Variables|Default|GetGridTileMarkers) (Math|Float|Truncate (+ (.x _output_get) (* (.y _output_get) (.x (Variables|Default|GetGridSize))))))))
      (bind _asbp_marker (Utilities|Casting|CastToBP_Marker (Variables|/Script/Engine.ChildActorComponent|GetChildActor _aschild_actor_component)))
      (Default|ActivateMarker _asbp_marker (Variables|Default|GetEditMode))
      (CallFunction|ChangeItemtoVisual (Variables|Default|GetDraggedItem) (Math|Vector2D|MakeVector2D (.x _output_get) (.y _output_get)))
      ;[0 0 0 1 34] HOVERED TILE CHANGED
      (if (Class|KismetMathLibrary|NotEqualExactlyVector2DVector2D (LocalVariables|GetTileInGrid) (Variables|Default|GetSelectedTile))
        ;[1 0 0 1 26] DEACTIVATE LAST TOUCHED TILE
        (CallFunction|DeactivateSelectedTile)
        (CallFunction|RevertItemVisual (Variables|Default|GetSelectedTile))
        (Variables|Default|SetSelectedTile (LocalVariables|GetTileInGrid))))))

(fn DeactivateSelectedTile
  (bind _selectedtile (Variables|Default|GetSelectedTile))
  ;[1 0.0498 0.2504 1 58] DEACTIVATE THE CURRENTLY SELECTED TILE
  (bind _aschild_actor_component (Utilities|Casting|CastToChildActorComponent (Components|GetChildComponent (Variables|Default|GetGridTileMarkers) (Math|Float|Truncate (+ (.x _selectedtile) (* (.y _selectedtile) (.x (Variables|Default|GetGridSize))))))))
  (bind _asbp_marker (Utilities|Casting|CastToBP_Marker (Variables|/Script/Engine.ChildActorComponent|GetChildActor _aschild_actor_component)))
  (Default|DeactivateMarker _asbp_marker))

(fn CreateBlankItem
  (params (Location :type Vector))
  ;[0.3248 0.1129 1 1 58] CREATE BLANK GRID ITEMS
  (bind _returnvalue (AddComponent|AddChildActorComponent false))
  (Transformation|AttachComponentToComponent _returnvalue (Variables|Default|GetGridTileItems) "None" "KeepRelative" "KeepRelative" "KeepRelative" true)
  (ChildActorComponent|SetChildActorClass _returnvalue "/Game/GameContent/Grid/GridObjects/BP_GridItem.BP_GridItem_C")
  (bind _asbp_grid_item (Utilities|Casting|CastToBP_GridItem (Variables|/Script/Engine.ChildActorComponent|GetChildActor _returnvalue)))
  (Default|UpdateItem _asbp_grid_item "NewEnumerator0")
  (Transformation|SetActorLocation _asbp_grid_item Location false false))

(fn ChangeItemtoVisual
  (params (Visual :type ENUM_ItemNames%20Enum :default "NewEnumerator0") (PositionInGrid :type Vector%202D%20Structure))
  ;[1 0 0 1 74] UPDATE GIVEN TILE TO MATCH GIVEN TYPE
  (bind _aschild_actor_component (Utilities|Casting|CastToChildActorComponent (Components|GetChildComponent (Variables|Default|GetGridTileItems) (Math|Float|Truncate (+ (.x PositionInGrid) (* (.y PositionInGrid) (.x (Variables|Default|GetGridSize))))))))
  (bind _asbp_grid_item (Utilities|Casting|CastToBP_GridItem (Variables|/Script/Engine.ChildActorComponent|GetChildActor _aschild_actor_component)))
  (bind _output_get (Variables|Default|SetCurrentTileBuildable _asbp_grid_item))
  (if (Utilities|Enum|Equal(Enum) (Variables|Default|GetEditMode) "NewEnumerator0")
    (Default|TempUpdateItem _output_get Visual)))

(fn RevertItemVisual
  (params (PositionInGrid :type Vector%202D%20Structure))
  ;[1 0 0 1 74] UPDATE GIVEN TILE TO MATCH GIVEN TYPE
  (bind _aschild_actor_component (Utilities|Casting|CastToChildActorComponent (Components|GetChildComponent (Variables|Default|GetGridTileItems) (Math|Float|Truncate (+ (.x PositionInGrid) (* (.y PositionInGrid) (.x (Variables|Default|GetGridSize))))))))
  (bind _asbp_grid_item (Utilities|Casting|CastToBP_GridItem (Variables|/Script/Engine.ChildActorComponent|GetChildActor _aschild_actor_component)))
  (bind _output_get (Variables|Default|SetCurrentTileBuildable _asbp_grid_item))
  (Default|UpdateItem _output_get (Variables|/Game/GameContent/Grid/GridObjects/BP_GridItem.BP_GridItem_C|GetItemType _output_get)))