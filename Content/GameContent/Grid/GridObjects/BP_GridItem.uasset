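; BP_GridItem is a grid object that displays an item whose type selects its data and mesh.
; On BeginPlay it calls UpdateItem with its ItemType, and the same function can switch it to another type.
; UpdateItem converts the enum value to a row name, looks up the data table, caches the row as ItemData and applies its ItemVisual to ObjectMesh.
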(event EventBeginPlay
  (CallFunction|UpdateItem (Variables|Default|GetItemType)))

(fn ConstructionScript)

(fn UpdateItem
  (params (ItemName :type ENUM_ItemNames%20Enum :default "NewEnumerator0"))
  (bind _output_get (Variables|Default|SetItemType ItemName))
  (bind _returnvalue (Utilities|GetDataTableRow (Variables|Default|GetDataTable) (Utilities|String|StringToName (Utilities|String|EnumtoString _output_get)))
    (:then
      (bind _output_get_2 (Variables|Default|SetItemData _returnvalue))
      (Components|StaticMesh|SetStaticMesh (Variables|Default|GetObjectMesh) (.itemvisual _output_get_2)))))