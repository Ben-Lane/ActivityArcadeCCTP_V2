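; Player data component on the top-down character that tracks steps, coins and tickets for a step-goal reward loop.
; BeginPlay derives a daily goal from average step history plus a share of the maximum.
; Step updates award coins at evenly spaced thresholds, coins convert into random ticket amounts for purchases, and changes update GameUI.
; EndPlay writes back to GI_PersistentData, but UpdatePlayerData currently returns the old values unchanged.
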(event Custom|UpdateCoins
  (params (UpdateAmount :type Integer))
  ;[1 1 1 1 58] UPDATE COINS VARIABLE + UI
  (Variables|Default|SetEarnedCoins (+ UpdateAmount (Variables|Default|GetEarnedCoins)))
  (Variables|Default|SetNormalCoins (+ UpdateAmount (Variables|Default|GetNormalCoins)))
  (bind _asbp_top_down_character (Utilities|Casting|CastToBP_TopDownCharacter (Components|GetOwner)))
  (bind _asbp_top_down_controller (Utilities|Casting|CastToBP_TopDownController (Pawn|GetController _asbp_top_down_character)))
  (Default|UpdateCoinsUI (Variables|/Game/TopDown/Blueprints/BP_TopDownController.BP_TopDownController_C|GetGameUI _asbp_top_down_controller) (Variables|Default|GetNormalCoins)))

(event Custom|StepsUpdated
  (params (UpdateAmount :type Integer))
  ;[1 1 1 1 50] UPDATE STEPS VARIABLES + UI
  (Variables|Default|SetUserSteps (+ UpdateAmount (Variables|Default|GetUserSteps)))
  (bind _asbp_top_down_character (Utilities|Casting|CastToBP_TopDownCharacter (Components|GetOwner)))
  (bind _asbp_top_down_controller (Utilities|Casting|CastToBP_TopDownController (Pawn|GetController _asbp_top_down_character)))
  (Default|UpdateStepUI (Variables|/Game/TopDown/Blueprints/BP_TopDownController.BP_TopDownController_C|GetGameUI _asbp_top_down_controller) (Variables|Default|GetUserSteps))
  (CallFunction|CheckCoinEarnings))

(event EventBeginPlay
  ;[0 0.2431 1 1 26] CALCULATE STEP GOAL ON OPEN
  (CallFunction|CalculateDailyStepGoal)
  (bind _asbp_top_down_character (Utilities|Casting|CastToBP_TopDownCharacter (Components|GetOwner)))
  (bind _asbp_top_down_controller (Utilities|Casting|CastToBP_TopDownController (Pawn|GetController _asbp_top_down_character)))
  (Default|UpdateCoinsUI (Variables|/Game/TopDown/Blueprints/BP_TopDownController.BP_TopDownController_C|GetGameUI _asbp_top_down_controller) (Variables|Default|GetNormalCoins)))

(event EventEndPlay
  (params (EndPlayReason :type EEndPlayReason%20Enum :default "Destroyed"))
  ;[1 0.02512 0 1 42] WHEN CLOSES, SAVE PLAYER DATA
  (bind _asgi_persistent_data (Utilities|Casting|CastToGI_PersistentData (Game|GetGameInstance)))
  (bind (_newstephistory _newtotalsteps _newtotaldistance) (CallFunction|UpdatePlayerData (.stephistory (Variables|/Game/GameContent/UserData/GI_PersistentData.GI_PersistentData_C|GetPlayerData _asgi_persistent_data)) (.totalsteps (Variables|/Game/GameContent/UserData/GI_PersistentData.GI_PersistentData_C|GetPlayerData _asgi_persistent_data)) (.totaldistance (Variables|/Game/GameContent/UserData/GI_PersistentData.GI_PersistentData_C|GetPlayerData _asgi_persistent_data))))
  (Variables|/Game/GameContent/UserData/GI_PersistentData.GI_PersistentData_C|SetPlayerData _asgi_persistent_data (Utilities|Struct|MakeS_PlayerData (.username (Variables|/Game/GameContent/UserData/GI_PersistentData.GI_PersistentData_C|GetPlayerData _asgi_persistent_data)) _newstephistory _newtotalsteps _newtotaldistance (.dailymaxgoal (Variables|/Game/GameContent/UserData/GI_PersistentData.GI_PersistentData_C|GetPlayerData _asgi_persistent_data)))))

(fn CalculateDailyStepGoal
  ;[0.6706 1 0.8988 1 50] Calculate the daily step goal of the user
  (bind _asgi_persistent_data (Utilities|Casting|CastToGI_PersistentData (Game|GetGameInstance)))
  (for _array_element (.stephistory (Variables|/Game/GameContent/UserData/GI_PersistentData.GI_PersistentData_C|GetPlayerData _asgi_persistent_data))
    (LocalVariables|SetTotalSteps (+ _array_element (LocalVariables|GetTotalSteps))))
  (bind _output_get (Variables|Default|SetDailyGoal (+ (/ (LocalVariables|GetTotalSteps) (Utilities|Array|Length (.stephistory (Variables|/Game/GameContent/UserData/GI_PersistentData.GI_PersistentData_C|GetPlayerData _asgi_persistent_data)))) (* (Math|Conversions|ToFloat(Integer) (.dailymaxgoal (Variables|/Game/GameContent/UserData/GI_PersistentData.GI_PersistentData_C|GetPlayerData _asgi_persistent_data))) (LocalVariables|GetMaxGoalPercentage)))))
  (return _output_get))

(fn UpdatePlayerData
  (params (OldStepHistory :type Array%20of%20Integers) (OldTotalSteps :type Integer) (OldTotalDistance :type Integer))
  ;[1 1 1] CURRENTLY DOESNT SAVE ANYTHING
  (return OldStepHistory OldTotalSteps OldTotalDistance))

(fn CheckCoinEarnings
  ;[1 0.1615 0.5327 1 34] GIVE PLAYER COINS FOR REACHING GOAL
  (if (not (Variables|Default|GetReachedMaximumCoins))
    (if (> (Variables|Default|GetUserSteps) (* (Math|Conversions|ToFloat(Integer) (+ (Variables|Default|GetEarnedCoins) 1)) (/ (Math|Conversions|ToFloat(Integer) (Variables|Default|GetDailyGoal)) (Variables|Default|GetCoinsAvailable))))
      (Development|PrintString "Earned Ticket")
      (CallFunction|UpdateCoins 1)
      (if (> (Variables|Default|GetUserSteps) (Variables|Default|GetDailyGoal))
        (Variables|Default|SetReachedMaximumCoins true)))))

(fn AddPlayerTickets
  (if (> (Variables|Default|GetNormalCoins) 0)
    (Variables|Default|SetNormalCoins (- (Variables|Default|GetNormalCoins) 1))
    (bind _output_get (LocalVariables|SetAddedTickets (Math|Random|RandomIntegerinRange 50 100)))
    (Variables|Default|SetTickets (+ (Variables|Default|GetTickets) _output_get))
    (bind _asbp_top_down_character (Utilities|Casting|CastToBP_TopDownCharacter (Components|GetOwner)))
    (bind _asbp_top_down_controller (Utilities|Casting|CastToBP_TopDownController (Pawn|GetController _asbp_top_down_character)))
    (Default|UpdateTicketsUI (Variables|/Game/TopDown/Blueprints/BP_TopDownController.BP_TopDownController_C|GetGameUI _asbp_top_down_controller) (Variables|Default|GetTickets))
    (Default|UpdateCoinsUI (Variables|/Game/TopDown/Blueprints/BP_TopDownController.BP_TopDownController_C|GetGameUI _asbp_top_down_controller) (Variables|Default|GetNormalCoins))
    (return true (LocalVariables|GetAddedTickets) 1)
    (else
      (return false 0 0))))

(fn MakeTicketPurchase
  (params (TicketsSpent :type Integer))
  ;[1 1 1] UPDATE TICKET PURCHASES
  (Variables|Default|SetTickets (- (Variables|Default|GetTickets) TicketsSpent))
  (bind _asbp_top_down_character (Utilities|Casting|CastToBP_TopDownCharacter (Components|GetOwner)))
  (bind _asbp_top_down_controller (Utilities|Casting|CastToBP_TopDownController (Pawn|GetController _asbp_top_down_character)))
  (Default|UpdateTicketsUI (Variables|/Game/TopDown/Blueprints/BP_TopDownController.BP_TopDownController_C|GetGameUI _asbp_top_down_controller) (Variables|Default|GetTickets)))